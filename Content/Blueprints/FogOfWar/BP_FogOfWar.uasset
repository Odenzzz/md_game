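; Fog of war Blueprint that draws a view area, supplied as a vertex array, into RT_FogOfWar2.
; BeginPlay creates two subtraction materials and clears both render targets.
; SubtractFromFog2 clears its target, pops the last vertex as player pivot, then draws material-driven triangles from pivot, PrevVertex (only set at index 0) and each later vertex.
; SubtractFromFog is empty; its location-and-size draw into RT_FogOfWar is disconnected.
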(event `self.ReceiveBeginPlay`
  (bind _returnvalue (`KismetMaterialLibrary.CreateDynamicMaterialInstance` "/Game/Materials/M_SubtractionOfFog.M_SubtractionOfFog"))
  (set `self.FogSubstruction` _returnvalue)
  (`KismetRenderingLibrary.ClearRenderTarget2D` "/Game/Textures/RT_FogOfWar.RT_FogOfWar")
  (bind _returnvalue_2 (`KismetMaterialLibrary.CreateDynamicMaterialInstance` "/Game/Materials/M_SubstractionOfFog2.M_SubstractionOfFog2"))
  (set `self.FogSubstruction2` _returnvalue_2)
  (`KismetRenderingLibrary.ClearRenderTarget2D` "/Game/Textures/RT_FogOfWar2.RT_FogOfWar2"))

(event `SubtractFromFog`
  (params (VectorConversion :type "Vector2D Structure") (Value :type "Float (double-precision)")))

(event `SubtractFromFog2`
  (params (viewAngleArray :type "Array of Vector2D Structure"))
  (bind _verticesarray (`self.verticesArray`))
  (bind _returnvalue (- (`KismetArrayLibrary.Array_Length` _verticesarray) 1))
  (set `self.verticesArray` viewAngleArray)
  (`|ExecutionSequence`
    (:`then_0`
      (`KismetRenderingLibrary.ClearRenderTarget2D` "/Game/Textures/RT_FogOfWar2.RT_FogOfWar2")
      ;[1 1 1] Pop player pivot vertex
      (set `self.playerFogPivot` (`|GetArrayItem` _verticesarray _returnvalue))
      (`KismetArrayLibrary.Array_Remove` (`self.verticesArray`) _returnvalue))
    (:`then_1`
      (for (_array_element _array_index) (`self.verticesArray`)
        (set `self.currentVertex` _array_element)
        (if (!= _array_index 0)
          (bind _value (`self.Convert Vertex` (`self.playerFogPivot`)))
          (`MaterialInstanceDynamic.SetVectorParameterValue` (`self.FogSubstruction2`) "PosB" _value)
          (bind _value_2 (`self.Convert Vertex` (`self.prevVertex`)))
          (`MaterialInstanceDynamic.SetVectorParameterValue` (`self.FogSubstruction2`) "PosA" _value_2)
          (bind _value_3 (`self.Convert Vertex` (`self.currentVertex`)))
          (`MaterialInstanceDynamic.SetVectorParameterValue` (`self.FogSubstruction2`) "PosC" _value_3)
          (`KismetRenderingLibrary.DrawMaterialToRenderTarget` "/Game/Textures/RT_FogOfWar2.RT_FogOfWar2" (`self.FogSubstruction2`))
          (else
            (set `self.prevVertex` (`self.currentVertex`))))))))

(fn `Convert Vertex`
  (params (vertex :type "Vector2D Structure"))
  (returns (value :type "LinearColor Structure"))
  (bind (_x _y) (`KismetMathLibrary.BreakVector2D` vertex))
  (return (`KismetMathLibrary.Conv_VectorToLinearColor` (`KismetMathLibrary.Conv_Vector2DToVector` (`KismetMathLibrary.MakeVector2D` _x _y)))))

(fn `UserConstructionScript`)