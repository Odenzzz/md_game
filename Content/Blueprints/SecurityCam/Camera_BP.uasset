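; Security camera actor that supplies a render-target view of what it captures.
; CreateInputView lazily creates a square render target with auto-generated mips on first call and assigns it as the CamView capture component's texture target.
; Later calls return the cached render target, while the event graph and construction script are empty.
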(fn `CreateInputView`
  (returns (RenderTarget :type "TextureRenderTarget2D Object Reference"))
  (if (not (`KismetSystemLibrary.IsValid` (`self.RenderTarget`)))
    (bind _returnvalue (`KismetRenderingLibrary.CreateRenderTarget2D` 1080 1080 "RTF_RGBA16f" (struct :`A` 1.0) true))
    (set `self.RenderTarget` _returnvalue)
    (set `SceneCaptureComponent2D.TextureTarget` _returnvalue (`self.CamView`))
    (return (`self.RenderTarget`))
    (else
      (return (`self.RenderTarget`)))))

(fn `UserConstructionScript`)