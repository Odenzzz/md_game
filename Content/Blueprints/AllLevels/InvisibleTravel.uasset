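; InvisibleTravel is an actor that seamlessly teleports whatever overlaps it to a matching destination in the level.
; On begin overlap, if a TargetPoint tag is set, it finds the first actor with that tag.
; It moves the overlapping actor there while keeping its offset from this trigger, so the jump can go unnoticed between identically built spaces.
; The overlapping actor is not filtered by type.
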(event `self.ReceiveActorBeginOverlap`
  (params (OtherActor :type "Actor Object Reference"))
  (if (!= (`self.TargetPoint`) "None")
    (set `self.TraveledPlayer` OtherActor)
    (bind _outactors (`GameplayStatics.GetAllActorsWithTag` (`self.TargetPoint`)))
    (`self.K2_SetActorLocation` (`self.TraveledPlayer`) (+ (`self.K2_GetActorLocation` (`|GetArrayItem` _outactors)) (- (`self.K2_GetActorLocation` (`self.TraveledPlayer`)) (`self.K2_GetActorLocation`))) false true)))

(fn `UserConstructionScript`)