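; Locked door Blueprint that starts a lockpicking minigame when the player interacts with it.
; Interact streams in the LockpickLevel2 sublevel if the door is unpicked and not in use, otherwise prints that it is already picked once OnPicked has set the flag.
; GetDifficulty returns a fixed difficulty enum value for this lock.
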(event `/Game/Blueprints/Gameplay/Lockpicking/LockpickInterface.OnPicked`
  (set `self.DoorPicked?` true))

(event `/Game/Blueprints/Character/Interaction_interface.Interact`
  (params (actor :type "Actor Object Reference") (player_controller :type "PlayerController Object Reference"))
  (if (not (`self.DoorPicked?`))
    (bind _isusing_ (`self.getIsUsing`))
    (if (not _isusing_)
      (`GameplayStatics.LoadStreamLevel` "LockpickLevel2" true))
    (else
      (`KismetSystemLibrary.PrintString` "Door already picked"))))

(fn `GetDifficulty`
  (returns (Difficulty :type "/Game/Blueprints/Gameplay/Lockpicking/LockpickDifficulty Enum"))
  (return "NewEnumerator0"))

(fn `UserConstructionScript`)