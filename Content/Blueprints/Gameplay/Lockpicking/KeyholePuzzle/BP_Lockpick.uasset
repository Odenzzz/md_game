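; Lockpick actor for the keyhole puzzle that slides a pick along its local Y axis from player input.
; The MoveLockpick axis input computes a speed-scaled Y position clamped between min and max limits, which Tick applies with a swept relative move.
; Its construction script restricts a SceneCaptureComponent2D to render only this actor's components.
; The RotateLockStop axis input is bound but does nothing.
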(event `InputAxis|MoveLockpick`
  (params (AxisValue :type "Float (single-precision)"))
  (set `self.LockpickPositionY` (`self.GetLockpickPosition` AxisValue)))

(event `InputAxis|RotateLockStop`
  (params (AxisValue :type "Float (single-precision)")))

(event `self.ReceiveTick`
  (params (DeltaSeconds :type "Float (single-precision)"))
  (`self.HandleTick` DeltaSeconds))

(fn `GetLockpickPosition`
  (params (PositionValue :type "Float (double-precision)"))
  (returns (NewParam :type "Float (double-precision)"))
  (locals (CurrentPositionY :type "Float (double-precision)" :default 0.0) (StartPosition :type "Vector Structure" :default (0.0 0.0 0.0)))
  (set `local.CurrentPositionY` (+ (* PositionValue (`self.LockpickMoveSpeed`)) (.y (`SceneComponent.RelativeLocation` (`self.Lockpick`)))))
  (`|ExecutionSequence`
    (:`then_0`
      (if (> (`local.CurrentPositionY`) (`self.MaxLockpickPositionY`))
        (set `local.CurrentPositionY` (`self.MaxLockpickPositionY`))))
    (:`then_1`
      (if (< (`local.CurrentPositionY`) (`self.MinLockpickPositionY`))
        (set `local.CurrentPositionY` (`self.MinLockpickPositionY`))))
    (:`then_2`
      (return (`local.CurrentPositionY`)))))

(fn `HandleTick`
  (params (DeltaSeconds :type "Float (double-precision)"))
  (`self.MoveLockpick`))

(fn `MoveLockpick`
  (`SceneComponent.K2_SetRelativeLocation` (`self.Lockpick`) (`KismetMathLibrary.MakeVector` (.x (`SceneComponent.RelativeLocation` (`self.Lockpick`))) (`self.LockpickPositionY`) (.z (`SceneComponent.RelativeLocation` (`self.Lockpick`)))) true false))

(fn `UserConstructionScript`
  (`SceneCaptureComponent.ShowOnlyActorComponents` (`self.SceneCaptureComponent2D`) self false))