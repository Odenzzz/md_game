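; Pin-tumbler lockpicking minigame actor that builds six randomly sized tumblers on BeginPlay and captures only itself via SceneCaptureComponent2D.
; Input slides and presses the pick, with Tick moving the current tumbler and spring, or shaking the lock when blocked.
; Tumblers set in array order within a narrow press window while the timeline-driven stopper is held; releasing it resets them.
; Setting all tumblers calls OnPicked and plays the opening animation.
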(event `self.ReceiveBeginPlay`
  (`self.GeneratePuzzle`))

(event `InputAction|LockpickPress`
  (params (Key :type "Key Structure"))
  (bind _returnvalue (not (`self.isOpened?`)))
  (:`Pressed`
    (if _returnvalue
      (set `self.isMovable?` false)
      (bind (_finded_ _tumbler) (`self.FindCurrentTumbler`))
      (set `self.hasCurrentTumbler?` _finded_)
      (set `self.currentTumbler` _tumbler)
      (set `self.isLockpickPressed?` true)
      (set `self.isLockpickUnpressing?` false)))
  (:`Released`
    (if _returnvalue
      (set `self.isLockpickUnpressing?` true))))

(event `InputAxis|MoveLockpick`
  (params (AxisValue :type "Float (single-precision)")))

(event `InputAxis|PressLockpick`
  (params (AxisValue :type "Float (single-precision)"))
  (set `self.lockpickPositionY` (`self.GetLockpickPosition` AxisValue))
  (set `self.lockpickPressingPercent` (`self.GetLockpickPressing` (- 0.0 AxisValue))))

(event `self.ReceiveTick`
  (params (DeltaSeconds :type "Float (single-precision)"))
  (if (not (`self.isOpened?`))
    (`self.HandleTick` DeltaSeconds)))

(event `InputAction|RotateLockStop`
  (params (Key :type "Key Structure"))
  (bind _returnvalue (not (`self.isOpened?`)))
  ;[1 1 1] Move stopper
  (:`Pressed`
    (if _returnvalue
      (switch `/Game/Blueprints/Gameplay/Lockpicking/LockpickStopStatus` (`self.StopperStatus`)
        (:`NewEnumerator2`
          _)
        (:`NewEnumerator3`
          _))
      (set `self.StopperStatus` "NewEnumerator0")
      (`self.MoveStopper`)))
  (:`Released`
    (if _returnvalue
      (switch `/Game/Blueprints/Gameplay/Lockpicking/LockpickStopStatus` (`self.StopperStatus`)
        (:`NewEnumerator0`
          _)
        (:`NewEnumerator1`
          _))
      (set `self.StopperStatus` "NewEnumerator2")
      (set `self.isStopped?` false)
      (set `self.isUnstopping?` true)
      (`self.MoveStopper`))))

(event `MoveStopper`
  ;[1 1 1] Move stopper
  (switch `/Game/Blueprints/Gameplay/Lockpicking/LockpickStopStatus` (`self.StopperStatus`)
    (:`NewEnumerator0`
      (bind (_direction _lockpickstop _lock) (`Timeline|OpenLock` :!label _label)
        (:`Update`
          (`SceneComponent.K2_SetRelativeRotation` (`self.lockpick_stop`) (`KismetMathLibrary.MakeRotator` 0.0 (+ (`self.StopperStartRotation`) (* (`self.StopperRotationAngle`) _lockpickstop))) false false)
          (`SceneComponent.K2_SetRelativeRotation` (`self.Lock`) (`KismetMathLibrary.MakeRotator` 0.0 (+ (`self.LockStartRotation`) (* (`self.ClosedLockRotateAngle`) _lock))) false false))
        (:`Finished`
          (switch `/Game/Blueprints/Gameplay/Lockpicking/LockpickStopStatus` (`self.StopperStatus`)
            (:`NewEnumerator0`
              (set `self.StopperStatus` "NewEnumerator1")
              (set `self.isStopped?` true))
            (:`NewEnumerator2`
              (set `self.StopperStatus` "NewEnumerator3")
              (set `self.isUnstopping?` false)
              (for (_array_element _array_index) (`self.tumblersArray`)
                (bind _structout (setmembers `/Game/Blueprints/Gameplay/Lockpicking/KeyholePuzzle/LockpickToggle_Structure` :`StructRef` _array_element :`isUnlocked?` false))
                (`KismetArrayLibrary.Array_Set` (`self.tumblersArray`) _array_index _structout)))))))
    (:`NewEnumerator1`
      (goto _label :!via `PlayFromStart`))
    (:`NewEnumerator2`
      (goto _label :!via `Reverse`))
    (:`NewEnumerator3`
      (goto _label :!via `ReverseFromEnd`))))

(event `PlayOpenAnimation`
  (bind (_direction _lockrotation) (`Timeline|OpenAnimation`)
    (:`Update`
      (`SceneComponent.K2_SetRelativeRotation` (`self.Lock`) (`KismetMathLibrary.MakeRotator` 0.0 (+ (`self.ClosedLockRotateAngle`) (* _lockrotation (`self.MaxLockRotateAngle`)))) false false))))

(event `ShakeLockpick`
  (bind (_relativerotation_roll _relativerotation_pitch) (`KismetMathLibrary.BreakRotator` (`SceneComponent.RelativeRotation` (`self.Lock`))))
  (if (and (`self.isShaking?`) (not (`self.ShakingPlaying`)))
    (set `self.currentShakeLockAngle` _relativerotation_pitch)
    (bind (_direction _shakevalue) (`Timeline|Shake` :!via `PlayFromStart`)
      (:`Update`
        (set `self.ShakingPlaying` true)
        (`SceneComponent.K2_SetRelativeRotation` (`self.Lock`) (`KismetMathLibrary.MakeRotator` 0.0 (+ (`self.currentShakeLockAngle`) (* (`self.lockShakeAngle`) _shakevalue))) false false))
      (:`Finished`
        (set `self.ShakingPlaying` false)))))

(fn `Check Lock Status`
  (returns (`Opened?` :type Boolean))
  (for _array_element (`self.tumblersArray`)
    (if (not (`.isUnlocked?_32_7D036DC44C96EC6EBA186EB27C74B49F` (break `/Game/Blueprints/Gameplay/Lockpicking/KeyholePuzzle/LockpickToggle_Structure` _array_element)))
      (return false)))
  (return true))

(fn `CheckPreviousTumblers`
  (returns (AllPreviousUnlocked :type Boolean))
  (for (_array_element _array_index) (`self.tumblersArray`)
    (if (== (`.Index_38_151324F843CFB72F0F9F18BAE18CAF31` (break `/Game/Blueprints/Gameplay/Lockpicking/KeyholePuzzle/LockpickToggle_Structure` (`self.currentTumbler`))) _array_index)
      (return true)
      (elif (not (`.isUnlocked?_32_7D036DC44C96EC6EBA186EB27C74B49F` (break `/Game/Blueprints/Gameplay/Lockpicking/KeyholePuzzle/LockpickToggle_Structure` _array_element)))
        (return false))))
  (return true))

(fn `FindCurrentTumbler`
  (returns (`finded?` :type Boolean) (tumbler :type "/Game/Blueprints/Gameplay/Lockpicking/KeyholePuzzle/LockpickToggle_Structure Structure"))
  (locals (tumblerSize :type "Float (double-precision)" :default 0.6) (lockpickTop :type "Float (double-precision)" :default 0.0))
  (bind _lockpicktop (`local.lockpickTop`))
  (set `local.lockpickTop` (- (`self.lockpickPositionY`) (`self.LockpickLength`)))
  (for _array_element (`self.tumblersArray`)
    (bind (_relativelocation_x _relativelocation_y) (`KismetMathLibrary.BreakVector` (`SceneComponent.RelativeLocation` (`.TumblerTop_12_65F12E9D4EE77731B25D96B208B477EA` (break `/Game/Blueprints/Gameplay/Lockpicking/KeyholePuzzle/LockpickToggle_Structure` _array_element)))))
    (if (and (> _lockpicktop (- _relativelocation_y (`local.tumblerSize`))) (< _lockpicktop (+ _relativelocation_y (`local.tumblerSize`))))
      (return true _array_element)))
  (return false))

(fn `GeneratePuzzle`
  (locals (TumblerHeightRange :type "Float (double-precision)" :default 1.25) (TumblerMaxScale :type "Float (double-precision)" :default 0.75) (SpringScaleRange :type "Float (double-precision)" :default 0.26) (SpringMaxScale :type "Float (double-precision)"))
  (`|ExecutionSequence`
    (:`then_0`
      (`|ExecutionSequence`
        (:`then_0`
          ;[1 1 1] Tumbler 1
          (`KismetArrayLibrary.Array_Add` (`self.tumblersArray`) (make `/Game/Blueprints/Gameplay/Lockpicking/KeyholePuzzle/LockpickToggle_Structure` (`KismetSystemLibrary.GetDisplayName` (`self.TumblerTop_1`)) 0 (`self.TumblerTop_1`) (`self.Spring_1_Top`) (`self.Spring_1`) 0.0 (`self.GetRandomScale`))))
        (:`then_1`
          ;[1 1 1] Tumbler 2
          (`KismetArrayLibrary.Array_Add` (`self.tumblersArray`) (make `/Game/Blueprints/Gameplay/Lockpicking/KeyholePuzzle/LockpickToggle_Structure` (`KismetSystemLibrary.GetDisplayName` (`self.TumblerTop_2`)) 0 (`self.TumblerTop_2`) (`self.Spring_2_Top`) (`self.Spring_2`) 0.0 (`self.GetRandomScale`))))
        (:`then_2`
          ;[1 1 1] Tumbler 3
          (`KismetArrayLibrary.Array_Add` (`self.tumblersArray`) (make `/Game/Blueprints/Gameplay/Lockpicking/KeyholePuzzle/LockpickToggle_Structure` (`KismetSystemLibrary.GetDisplayName` (`self.TumblerTop_3`)) 0 (`self.TumblerTop_3`) (`self.Spring_3_Top`) (`self.Spring_3`) 0.0 (`self.GetRandomScale`))))
        (:`then_3`
          ;[1 1 1] Tumbler 4
          (`KismetArrayLibrary.Array_Add` (`self.tumblersArray`) (make `/Game/Blueprints/Gameplay/Lockpicking/KeyholePuzzle/LockpickToggle_Structure` (`KismetSystemLibrary.GetDisplayName` (`self.TumblerTop_4`)) 0 (`self.TumblerTop_4`) (`self.Spring_4_Top`) (`self.Spring_4`) 0.0 (`self.GetRandomScale`))))
        (:`then_4`
          ;[1 1 1] Tumbler 5
          (`KismetArrayLibrary.Array_Add` (`self.tumblersArray`) (make `/Game/Blueprints/Gameplay/Lockpicking/KeyholePuzzle/LockpickToggle_Structure` (`KismetSystemLibrary.GetDisplayName` (`self.TumblerTop_5`)) 0 (`self.TumblerTop_5`) (`self.Spring_5_Top`) (`self.Spring_5`) 0.0 (`self.GetRandomScale`))))
        (:`then_5`
          ;[1 1 1] Tumbler 6
          (`KismetArrayLibrary.Array_Add` (`self.tumblersArray`) (make `/Game/Blueprints/Gameplay/Lockpicking/KeyholePuzzle/LockpickToggle_Structure` (`KismetSystemLibrary.GetDisplayName` (`self.TumblerTop_6`)) 0 (`self.TumblerTop_6`) (`self.Spring_6_Top`) (`self.Spring_6`) 0.0 (`self.GetRandomScale`))))))
    (:`then_1`
      (for (_array_element _array_index) (`self.tumblersArray`)
        (`|ExecutionSequence`
          (:`then_0`
            (bind _returnvalue (- (`local.TumblerHeightRange`) (* (/ (`local.TumblerHeightRange`) (`local.TumblerMaxScale`)) (- (`.Scale_20_D6664F224CED566DCE1309AED433DCA7` (break `/Game/Blueprints/Gameplay/Lockpicking/KeyholePuzzle/LockpickToggle_Structure` _array_element)) 1.0))))
            (bind _structout (setmembers `/Game/Blueprints/Gameplay/Lockpicking/KeyholePuzzle/LockpickToggle_Structure` :`StructRef` _array_element :`Index` _array_index :`ScaleValue` _returnvalue :`Locked_TumblerTopPosition` (+ (`self.TumblerTopStartPosition`) _returnvalue) :`Locked_SpringTopPosition` (+ (`self.SpringTopStartPosition`) _returnvalue) :`Locked_SpringScale` (+ (* (`local.SpringScaleRange`) _returnvalue) (`self.SpringStartScale`)) :`UnlockRangeStart` _returnvalue))
            (`KismetArrayLibrary.Array_Set` (`self.tumblersArray`) _array_index _structout))
          (:`then_1`
            (`self.SetTumblerPosition` (`|GetArrayItem` (`self.tumblersArray`) _array_index))))))))

(fn `getCompressedValue`
  (params (Current :type "Float (double-precision)") (Delta :type "Float (double-precision)") (Target :type "Float (double-precision)"))
  (returns (Value :type "Float (double-precision)"))
  (bind _returnvalue (+ Current Delta))
  (if (> _returnvalue Target)
    (return Target)
    (else
      (return _returnvalue))))

(fn `GetLockpickPosition`
  (params (PositionValue :type "Float (double-precision)"))
  (returns (LockpickPositionY :type "Float (double-precision)"))
  (locals (CurrentPositionY :type "Float (double-precision)" :default 0.0) (StartPosition :type "Vector Structure" :default (0.0 0.0 0.0)))
  (if (`self.isMovable?`)
    (set `local.CurrentPositionY` (+ (* PositionValue (`self.LockpickMoveSpeed`)) (.y (`SceneComponent.RelativeLocation` (`self.lockpick`)))))
    (`|ExecutionSequence`
      (:`then_0`
        (if (> (`local.CurrentPositionY`) (`self.MaxLockpickPositionY`))
          (set `local.CurrentPositionY` (`self.MaxLockpickPositionY`))))
      (:`then_1`
        (if (< (`local.CurrentPositionY`) (`self.MinLockpickPositionY`))
          (set `local.CurrentPositionY` (`self.MinLockpickPositionY`))))
      (:`then_2`
        (return (`local.CurrentPositionY`))))
    (else
      (return (`self.lockpickPositionY`)))))

(fn `GetLockpickPressing`
  (params (Value :type "Float (double-precision)"))
  (returns (Percent :type "Float (double-precision)"))
  (locals (PressSpeed :type "Float (double-precision)" :default 0.2))
  (if (`self.isLockpickPressed?`)
    (set `self.lockpickPressingPercent` (+ (`self.lockpickPressingPercent`) (* Value (`local.PressSpeed`))))
    (if (> (`self.lockpickPressingPercent`) 1.0)
      (bind _output_get (set `self.lockpickPressingPercent` 1.0))
      (return _output_get)
      (elif (< (`self.lockpickPressingPercent`) 0.0)
        (bind _output_get_2 (set `self.lockpickPressingPercent` 0.0))
        (return _output_get_2)
        (else
          (return (`self.lockpickPressingPercent`)))))))

(fn `GetRandomScale`
  (returns (Scale :type "Float (double-precision)"))
  (locals (Precision :type "Float (double-precision)" :default 100.0))
  (return (/ (`KismetMathLibrary.Conv_IntToDouble` (`KismetMathLibrary.FFloor` (* (`KismetMathLibrary.RandomFloatInRange` 1.0 1.6) (`local.Precision`)))) (`local.Precision`))))

(fn `HandleTick`
  (params (DeltaSeconds :type "Float (double-precision)"))
  (locals (DT :type "Float (double-precision)"))
  (bind _output_get (set `local.DT` DeltaSeconds))
  (`|ExecutionSequence`
    (:`then_0`
      (if (and (`self.isLockpickUnpressing?`) (> (`self.lockpickPressingPercent`) 0.0))
        (set `self.lockpickPressingPercent` (`self.GetLockpickPressing` (- 0.0 (* _output_get 100.0))))
        (elif (and (`self.isLockpickUnpressing?`) (== (`self.lockpickPressingPercent`) 0.0))
          (set `self.isLockpickPressed?` false)
          (set `self.isMovable?` true)
          (set `self.hasCurrentTumbler?` false)
          (set `self.isLockpickUnpressing?` false))))
    (:`then_1`
      (if (`self.isUnstopping?`)
        (for _array_element (`self.tumblersArray`)
          (bind (_tumblername _index _tumblertop _springtop _spring _scalevalue _scale _locked_tumblertopposition _locked_springtopposition _locked_springscale _unlockrangestart _isunlocked_) (break `/Game/Blueprints/Gameplay/Lockpicking/KeyholePuzzle/LockpickToggle_Structure` _array_element))
          (if _isunlocked_
            (bind (_relativelocation_x _relativelocation_y _relativelocation_z) (`KismetMathLibrary.BreakVector` (`SceneComponent.RelativeLocation` _tumblertop)))
            (`SceneComponent.K2_SetRelativeLocation` _tumblertop (`KismetMathLibrary.MakeVector` _relativelocation_x _relativelocation_y (`self.getCompressedValue` _relativelocation_z (* (`local.DT`) 30.0) _locked_tumblertopposition)) false false)
            (bind (_relativelocation_x_2 _relativelocation_y_2 _relativelocation_z_2) (`KismetMathLibrary.BreakVector` (`SceneComponent.RelativeLocation` _springtop)))
            (`SceneComponent.K2_SetRelativeLocation` _springtop (`KismetMathLibrary.MakeVector` _relativelocation_x_2 _relativelocation_y_2 (`self.getCompressedValue` _relativelocation_z_2 (* (`local.DT`) 30.0) _locked_springtopposition)) false false)
            (bind (_relativescale3d_x _relativescale3d_y _relativescale3d_z) (`KismetMathLibrary.BreakVector` (`SceneComponent.RelativeScale3D` _spring)))
            (`SceneComponent.SetRelativeScale3D` _spring (`KismetMathLibrary.MakeVector` _relativescale3d_x _relativescale3d_y (`self.getCompressedValue` _relativescale3d_z (* (`local.DT`) 30.0) _locked_springscale)))))))
    (:`then_2`
      (`self.MoveLockpick`)
      (`self.PressLockpick`)
      (`self.ShakeLockpick`))))

(fn `LockpickPressing`)

(fn `MoveLockpick`
  (`SceneComponent.K2_SetRelativeLocation` (`self.lockpick`) (`KismetMathLibrary.MakeVector` (.x (`SceneComponent.RelativeLocation` (`self.lockpick`))) (`self.lockpickPositionY`) (.z (`SceneComponent.RelativeLocation` (`self.lockpick`)))) true false))

(fn `PressLockpick`
  (locals (PressAngle :type "Float (double-precision)" :default -5.3) (PressMoveY :type "Float (double-precision)" :default -0.077) (PressMoveZ :type "Float (double-precision)" :default 0.874) (lockpickStartAngle :type "Float (double-precision)" :default 270.0) (lockpickStartPositionZ :type "Float (double-precision)" :default 1.7) (TumblerPressingPrecent :type "Float (double-precision)" :default 0.22) (TumblerPressingRange :type "Float (double-precision)" :default 1.5) (TumblerPressedRange :type "Float (double-precision)" :default 0.0) (SpringScaleRange :type "Float (double-precision)" :default 0.36) (SpringScaledRange :type "Float (double-precision)"))
  (bind (_tumblername _index _tumblertop _springtop _spring _scalevalue _scale _locked_tumblertopposition _locked_springtopposition _locked_springscale _unlockrangestart _isunlocked_) (break `/Game/Blueprints/Gameplay/Lockpicking/KeyholePuzzle/LockpickToggle_Structure` (`self.currentTumbler`)))
  (bind _returnvalue (/ (- (`self.lockpickPressingPercent`) (`local.TumblerPressingPrecent`)) (- 1.0 (`local.TumblerPressingPrecent`))))
  (bind (_relativelocation_x _relativelocation_y) (`KismetMathLibrary.BreakVector` (`SceneComponent.RelativeLocation` _tumblertop)))
  (bind (_relativelocation_x_2 _relativelocation_y_2) (`KismetMathLibrary.BreakVector` (`SceneComponent.RelativeLocation` _springtop)))
  (if (`self.isLockpickPressed?`)
    (if (`self.hasCurrentTumbler?`)
      (set `local.PressAngle` -6.5)
      (set `local.PressMoveZ` 1.1)
      (set `local.PressMoveY` -0.4)
      (if (or (`self.CheckPreviousTumblers`) (< (`self.lockpickPressingPercent`) 0.59))
        (set `self.isShaking?` false :!label _label)
        (`SceneComponent.K2_SetRelativeLocationAndRotation` (`self.lockpick`) (`KismetMathLibrary.MakeVector` -0.05 (+ (`self.lockpickPositionY`) (* (`local.PressMoveY`) (`self.lockpickPressingPercent`))) (+ (`local.lockpickStartPositionZ`) (* (`local.PressMoveZ`) (`self.lockpickPressingPercent`)))) (`KismetMathLibrary.MakeRotator` (+ (`local.lockpickStartAngle`) (* (`local.PressAngle`) (`self.lockpickPressingPercent`)))) false false)
        (if (`self.hasCurrentTumbler?`)
          (if (> (`self.lockpickPressingPercent`) (`local.TumblerPressingPrecent`))
            (set `local.TumblerPressedRange` (* _returnvalue (`local.TumblerPressingRange`)))
            (set `local.SpringScaledRange` (* (`local.SpringScaleRange`) _returnvalue))
            (else
              (set `local.TumblerPressedRange` 0.0)
              (set `local.SpringScaledRange` 0.0)))
          (`|ExecutionSequence`
            (:`then_0`
              (if (not (and (< (`local.TumblerPressedRange`) _unlockrangestart) _isunlocked_))
                (`SceneComponent.K2_SetRelativeLocation` _tumblertop (`KismetMathLibrary.MakeVector` _relativelocation_x _relativelocation_y (- _locked_tumblertopposition (`local.TumblerPressedRange`))) false false)
                (`SceneComponent.K2_SetRelativeLocation` _springtop (`KismetMathLibrary.MakeVector` _relativelocation_x_2 _relativelocation_y_2 (- _locked_springtopposition (`local.TumblerPressedRange`))) false false)
                (`SceneComponent.SetRelativeScale3D` _spring (`KismetMathLibrary.MakeVector` 1.0 1.0 (- _locked_springscale (`local.SpringScaledRange`))))))
            (:`then_1`
              (if (not (`self.isLockpickUnpressing?`))
                (if (and (or (and _isunlocked_ (< (`local.TumblerPressedRange`) _unlockrangestart)) (and (> (`local.TumblerPressedRange`) _unlockrangestart) (< (`local.TumblerPressedRange`) (+ _unlockrangestart 0.1)))) (`self.isStopped?`))
                  (bind _structout (setmembers `/Game/Blueprints/Gameplay/Lockpicking/KeyholePuzzle/LockpickToggle_Structure` :`StructRef` (`self.currentTumbler`) :`isUnlocked?` true))
                  (`KismetArrayLibrary.Array_Set` (`self.tumblersArray`) (`.Index_38_151324F843CFB72F0F9F18BAE18CAF31` (break `/Game/Blueprints/Gameplay/Lockpicking/KeyholePuzzle/LockpickToggle_Structure` _structout)) _structout)
                  (if (`self.Check Lock Status`)
                    (set `self.isOpened?` true)
                    (`self.OnPicked`)
                    (`self.PlayOpenAnimation`))
                  (else
                    (bind _structout_2 (setmembers `/Game/Blueprints/Gameplay/Lockpicking/KeyholePuzzle/LockpickToggle_Structure` :`StructRef` (`self.currentTumbler`) :`isUnlocked?` false))
                    (`KismetArrayLibrary.Array_Set` (`self.tumblersArray`) (`.Index_38_151324F843CFB72F0F9F18BAE18CAF31` (break `/Game/Blueprints/Gameplay/Lockpicking/KeyholePuzzle/LockpickToggle_Structure` _structout_2)) _structout_2)))))))
        (else
          (set `self.isShaking?` true :!label _label_2)))
      (else
        (set `local.PressAngle` -5.3)
        (set `local.PressMoveZ` 0.874)
        (set `local.PressMoveY` -0.077)
        (if (< (`self.lockpickPressingPercent`) 0.95)
          (goto _label)
          (else
            (goto _label_2)))))))

(fn `SetTumblerPosition`
  (params (Tumbler :type "/Game/Blueprints/Gameplay/Lockpicking/KeyholePuzzle/LockpickToggle_Structure Structure"))
  (bind (_tumblername _index _tumblertop _springtop _spring _scalevalue _scale _locked_tumblertopposition _locked_springtopposition _locked_springscale) (break `/Game/Blueprints/Gameplay/Lockpicking/KeyholePuzzle/LockpickToggle_Structure` Tumbler))
  (`|ExecutionSequence`
    (:`then_0`
      (`SceneComponent.K2_SetRelativeLocation` _tumblertop (`KismetMathLibrary.MakeVector` (.x (`SceneComponent.RelativeLocation` _tumblertop)) (.y (`SceneComponent.RelativeLocation` _tumblertop)) _locked_tumblertopposition) false false)
      (`SceneComponent.SetRelativeScale3D` _tumblertop (`KismetMathLibrary.MakeVector` 1.0 1.0 _scale)))
    (:`then_1`
      (`SceneComponent.K2_SetRelativeLocation` _springtop (`KismetMathLibrary.MakeVector` (.x (`SceneComponent.RelativeLocation` _springtop)) (.y (`SceneComponent.RelativeLocation` _springtop)) _locked_springtopposition) false false))
    (:`then_2`
      (`SceneComponent.SetRelativeScale3D` _spring (`KismetMathLibrary.MakeVector` (.x (`SceneComponent.RelativeScale3D` _spring)) (.y (`SceneComponent.RelativeScale3D` _spring)) _locked_springscale)))))

(fn `UserConstructionScript`
  (`SceneCaptureComponent.ShowOnlyActorComponents` (`self.SceneCaptureComponent2D`) self false))