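; Base player character Blueprint with control-yaw-relative movement, idle/walk animation switching and an interact action.
; Interact line-traces ahead, messages the hit actor and, if it casts to an unused UsableComponent, assigns the player controller as owner via server and multicast events.
; MoveForward uses the right vector and MoveRight the forward one.
; Tick's rotation replication ends in an empty event, UpdateAnimation is never called here, and deprecated 2D movement is disconnected.
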(event `self.ReceiveBeginPlay`
  (set `PlayerController.bShowMouseCursor` false (`GameplayStatics.GetPlayerController` 0)))

(event `UpdateAnimation`
  ;[1 1 1] Handle Animation
  (`SkeletalMeshComponent.SetAnimation` (`self.Mesh`) (select `bool` (> (`KismetMathLibrary.VSize` (`self.GetVelocity`)) 0.0) :`false` "/Game/Models/Character/Animations/CharacterIdle.CharacterIdle" :`true` "/Game/Models/Character/Animations/CharacterWalk.CharacterWalk" :!type "AnimationAsset Object Reference")))

(event `InputAxis|MoveForward`
  (params (AxisValue :type "Float (single-precision)"))
  ;[1 1 1] Handle movement
  (`self.AddMovementInput` (`KismetMathLibrary.GetRightVector` (`KismetMathLibrary.MakeRotator` 0.0 0.0 (.yaw (`self.GetControlRotation`)))) AxisValue))

(event `InputAxis|MoveRight`
  (params (AxisValue :type "Float (single-precision)"))
  ;[1 1 1] Handle movement
  (`self.AddMovementInput` (`KismetMathLibrary.GetForwardVector` (`KismetMathLibrary.MakeRotator` 0.0 0.0 (.yaw (`self.GetControlRotation`)))) AxisValue))

(event `InputAction|InteractEvent`
  (params (Key :type "Key Structure"))
  (bind _returnvalue (`GameplayStatics.GetPlayerController` 0))
  (bind _returnvalue_2 (`self.K2_GetActorLocation`))
  (bind _yaw (.yaw (`self.K2_GetActorRotation`)))
  ;[1 1 1] interaction
  (:`Pressed`
    (bind (_outhit _returnvalue_3) (`KismetSystemLibrary.LineTraceSingle` :`Start` _returnvalue_2 :`End` (+ _returnvalue_2 (`KismetMathLibrary.MakeVector` (* (`KismetMathLibrary.DegCos` _yaw) 140.0) (* (`KismetMathLibrary.DegSin` _yaw) 140.0) 0.0)) :`TraceChannel` "TraceTypeQuery1" :`DrawDebugType` "ForDuration"))
    (if _returnvalue_3
      (bind (_bblockinghit _binitialoverlap _time _distance _location _impactpoint _normal _impactnormal _physmat _hitactor) (`GameplayStatics.BreakHitResult` _outhit))
      (message `/Game/Blueprints/Character/Interaction_interface.Interact` _hitactor self _returnvalue)
      (bind _asusable_component (cast `/Game/Blueprints/UsableComponent` _hitactor))
      (if (not (`/Game/Blueprints/UsableComponent.IsUsing?` _asusable_component))
        (`self.SetOwnerEvent` _hitactor _returnvalue)))))

(event `self.ReceiveTick`
  (params (DeltaSeconds :type "Float (single-precision)"))
  ;[1 1 1] Tick - Updates animation
  (`/Engine/EditorBlueprintResources/ActorMacros.Switch Has Authority`
    (:`Authority`
      (`self.Movement_rotation_multi`))
    (:`Remote`
      (`self.Movement_rotation_on_server`))))

(event `Movement_rotation_on_server`
  ;[1 1 1] Tick - Updates animation
  (`self.Movement_rotation_multi`))

(event `Movement_rotation_multi`
  ;[1 1 1] Tick - Updates animation
)

(event `SetOwnerEvent`
  (params (Target :type "Actor Object Reference") (Player :type "Actor Object Reference"))
  ;[1 1 1] interaction
  (`/Engine/EditorBlueprintResources/ActorMacros.Switch Has Authority`
    (:`Authority`
      (`self.SetOwner_Multi` Target Player))
    (:`Remote`
      (`self.SetOwner_Server` Target Player))))

(event `SetOwner_Server`
  (params (Target :type "Actor Object Reference") (Player :type "Actor Object Reference"))
  ;[1 1 1] interaction
  (`self.SetOwner_Multi` Target Player))

(event `SetOwner_Multi`
  (params (Target :type "Actor Object Reference") (Player :type "Actor Object Reference"))
  ;[1 1 1] interaction
  (`self.SetOwner` Target Player))

(event `MoveMulti`
  ;[1 1 1] Handle movement 2d (deplecated)
)

(event `MoveOnServer`
  ;[1 1 1] Handle movement 2d (deplecated)
  (`self.MoveMulti`))

(fn `Interact`
  (params (actor :type "Actor Object Reference") (player_controller :type "PlayerController Object Reference"))
  (return))

(fn `UserConstructionScript`)