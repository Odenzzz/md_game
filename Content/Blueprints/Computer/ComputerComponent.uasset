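; Actor component for an in-game computer that shows a desktop widget on its screen and opens a viewport copy when a player interacts.
; On BeginPlay it numbers installed programs by array index and creates the screen widget at 1080p.
; Interact creates a viewport-sized widget, then after a short delay switches to UI-only input with a cursor.
; Program moves route through server and multicast events to update the Computer struct and refresh the screen widget.
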(event `/Game/Blueprints/Character/Interaction_interface.Interact`
  (params (actor :type "Actor Object Reference") (player_controller :type "PlayerController Object Reference"))
  (bind _returnvalue (`GameplayStatics.GetPlayerController` 0))
  (bind _output_get (set `self.PlayerController` player_controller))
  (if (not (`self.IsUsing?`))
    (bind (_sizex _sizey) (`PlayerController.GetViewportSize` _output_get))
    (bind _computerwidget (`self.ToggleComputerWidget` (`KismetMathLibrary.MakeVector2D` (`KismetMathLibrary.Conv_IntToDouble` _sizex) (`KismetMathLibrary.Conv_IntToDouble` _sizey))))
    (set `self.ComputerWidget` _computerwidget)
    (`UserWidget.AddToViewport` (`self.ComputerWidget`) 0)
    ;[1 1 1] delay for character stop moving
    (`KismetSystemLibrary.Delay` 0.3)
    (`WidgetBlueprintLibrary.SetInputMode_UIOnlyEx` _returnvalue (`self.ComputerWidget`))
    (set `PlayerController.bShowMouseCursor` true _returnvalue)
    (`self.TurnIsUsing` true)))

(event `self.ReceiveBeginPlay`
  ;[1 1 1] Init
  (`self.SetProgramsIDs`)
  (bind _computerwidget (`self.ToggleComputerWidget` (1920.0 1080.0)))
  (bind _output_get (set `self.ComputerScreenWidget` _computerwidget))
  (set `self.ComputerWidget` _computerwidget)
  (`WidgetComponent.SetWidget` (`self.ComputerScreen`) _output_get))

(event `SetProgramsIDs`
  (bind _computer (`self.Computer`))
  (for (_array_element _array_index) (`.InstalledProgramsStructure_12_9A8DF5174E5EFB7F80F70B8A013D8AC7` (break `/Game/Blueprints/Computer/ComputerStructure` _computer))
    (bind _structout (setmembers `/Game/Blueprints/Computer/Programs/Program/ProgramStructure` :`StructRef` (`.ProgramStructure_4_F417B182435403B8CBF594829B8150D8` (break `/Game/Blueprints/Computer/Programs/InstalledProgramsStructure` _array_element)) :`ID` _array_index))
    (bind _structout_2 (setmembers `/Game/Blueprints/Computer/Programs/InstalledProgramsStructure` :`StructRef` _array_element :`ProgramStructure` _structout))
    (`KismetArrayLibrary.Array_Add` (`self.InstalledProgramsContainer`) _structout_2))
  (setmembers `/Game/Blueprints/Computer/ComputerStructure` :`StructRef` _computer :`InstalledProgramsStructure` (`self.InstalledProgramsContainer`)))

(event `ChangeProgramPosition`
  (params (ProgramPosition :type "/Game/Blueprints/Computer/Programs/Program/ProgramPositionStructure Structure") (ProgramID :type Integer))
  ;[1 1 1] Update program position
  (`|ExecutionSequence`
    (:`then_0`
      (`/Engine/EditorBlueprintResources/ActorMacros.Switch Has Authority`
        (:`Authority`
          (`self.ChangeProgramPosition_Multi` ProgramPosition ProgramID))
        (:`Remote`
          (`self.ChangeProgramPosition_Server` ProgramPosition ProgramID))))))

(event `ChangeProgramPosition_Server`
  (params (ProgramPosition :type "/Game/Blueprints/Computer/Programs/Program/ProgramPositionStructure Structure") (ProgramID :type Integer))
  ;[1 1 1] Update program position
  (`self.ChangeProgramPosition_Multi` ProgramPosition ProgramID))

(event `ChangeProgramPosition_Multi`
  (params (ProgramPosition :type "/Game/Blueprints/Computer/Programs/Program/ProgramPositionStructure Structure") (ProgramID :type Integer))
  (bind _installedprogramscontainer (`self.InstalledProgramsContainer`))
  (bind _computer (`self.Computer`))
  ;[1 1 1] Update program position
  (for (_array_element _array_index) (`.InstalledProgramsStructure_12_9A8DF5174E5EFB7F80F70B8A013D8AC7` (break `/Game/Blueprints/Computer/ComputerStructure` _computer))
    (bind _programstructure (break `/Game/Blueprints/Computer/Programs/InstalledProgramsStructure` _array_element))
    (if (== ProgramID (`.ID_42_D1E2B9044B1EA92F1E1BC5BEF8B2F5CA` (break `/Game/Blueprints/Computer/Programs/Program/ProgramStructure` _programstructure)))
      (bind _structout (setmembers `/Game/Blueprints/Computer/Programs/Program/ProgramStructure` :`StructRef` _programstructure :`PositionData` ProgramPosition))
      (bind _structout_2 (setmembers `/Game/Blueprints/Computer/Programs/InstalledProgramsStructure` :`StructRef` _array_element :`ProgramStructure` _structout))
      (`KismetArrayLibrary.Array_Set` _installedprogramscontainer _array_index _structout_2 true)
      (else
        (`KismetArrayLibrary.Array_Set` _installedprogramscontainer _array_index _array_element true))))
  (setmembers `/Game/Blueprints/Computer/ComputerStructure` :`StructRef` _computer :`InstalledProgramsStructure` (`self.InstalledProgramsContainer`))
  ;;[1 1 1] Update program positions on computer block
  (`/Game/UI/Computer/Computer.UpdatePrograms` (`self.ComputerScreenWidget`) (`self.Computer`) (`self.ComputerScreenWidget`) (1920.0 1080.0)))

(fn `ToggleComputerWidget`
  (params (WindowSize :type "Vector2D Structure"))
  (returns (ComputerWidget :type "/Game/UI/Computer/Computer Object Reference"))
  (bind _returnvalue (`|CreateWidget` "/Game/UI/Computer/Computer.Computer_C" null self (`self.Computer`) WindowSize))
  (return _returnvalue))

(fn `UserConstructionScript`)